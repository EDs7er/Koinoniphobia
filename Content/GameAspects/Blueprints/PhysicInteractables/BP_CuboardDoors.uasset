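; Physics-driven cupboard with left and right doors that swing in response to hand interaction on their knobs.
; The Interact event matches the touched component to the left knob by object name, treating any other as the right side.
; It applies a force at that component's location to the matching door, scaled from the hand-to-component offset.
; The left door's force points away from the hand, while the right door's points toward it.
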(event `/Game/GameAspects/Blueprints/PhysicInteractables/PhysicObjectInterface.Interact`
  (params (HandLocation :type "Vector Structure") (Component :type "SceneComponent Object Reference"))
  (bind _returnvalue (`SceneComponent.K2_GetComponentLocation` Component))
  (if (`KismetStringLibrary.EqualEqual_StrStr` (`KismetSystemLibrary.GetObjectName` Component) (`KismetSystemLibrary.GetObjectName` (`self.KnobLeft`)))
    (`PrimitiveComponent.AddForceAtLocation` (`self.IO_Cupboard_04_Door_Left`) (* (- _returnvalue HandLocation) 50.0) _returnvalue "None")
    (else
      (`PrimitiveComponent.AddForceAtLocation` (`self.IO_Cupboard_04_Door_Right`) (* (- HandLocation _returnvalue) 50.0) _returnvalue "None"))))

(fn `UserConstructionScript`)