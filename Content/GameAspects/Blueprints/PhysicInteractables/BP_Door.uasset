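; BP_Door is a lockable physics door that players pull by hand using motion controllers.
; Each tick it checks the Lock component's overlaps for a "Key"-tagged component, then makes motion controllers release their held actors, unlocks, and destroys the key after a short delay.
; While unlocked, Interact applies force to the Door at the interacted component's location, scaled by that component's offset to the hand.
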(event `self.ReceiveTick`
  (params (DeltaSeconds :type "Float (single-precision)"))
  ;[1 1 1] Drops key/Unlocks door/destroys ke
  (for _array_element (`PrimitiveComponent.GetOverlappingComponents` (`self.Lock`))
    (if (`ActorComponent.ComponentHasTag` _array_element "Key")
      (bind _outactors (`GameplayStatics.GetAllActorsOfClass` "/Game/GameAspects/Blueprints/BP_MotionController.BP_MotionController_C"))
      (for _array_element_2 _outactors
        (bind _asbp_motion_controller (cast `/Game/GameAspects/Blueprints/BP_MotionController` _array_element_2))
        (`/Game/GameAspects/Blueprints/BP_MotionController.ReleaseActor` _asbp_motion_controller)
        (set `self.Locked?` false)
        (bind _asbp_key_child (cast `/Game/GameAspects/Blueprints/Interactables/BP_Key_Child` (`ActorComponent.GetOwner` _array_element)))
        (`KismetSystemLibrary.Delay` 0.1)
        (`self.K2_DestroyActor` _asbp_key_child)))))

(event `/Game/GameAspects/Blueprints/PhysicInteractables/PhysicObjectInterface.Interact`
  (params (HandLocation :type "Vector Structure") (Component :type "SceneComponent Object Reference"))
  (bind _returnvalue (`SceneComponent.K2_GetComponentLocation` Component))
  (if (not (`self.Locked?`))
    (`PrimitiveComponent.AddForceAtLocation` (`self.Door`) (* (- HandLocation _returnvalue) 50.0) _returnvalue "None")))

(fn `UserConstructionScript`)