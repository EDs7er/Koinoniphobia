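; BP_GunInteractable is a VR gun that can be picked up, dropped and fired.
; BP_MotionController calls Pickup, which disables physics and snaps the skeletal mesh to the given component with small rotation and position corrections; Drop re-enables physics and detaches.
; FireGun plays animation, sound and muzzle effect, then scans HitBox overlaps, matching one hard-coded VRPawn headset display name to shove that pawn along world -X.
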(event `FireGun`
  (`SkeletalMeshComponent.PlayAnimation` (`self.SkeletalMesh`) "/Game/Geometry/Meshes/Misc/IO_GunRigged_01_Anim.IO_GunRigged_01_Anim" false)
  (`GameplayStatics.PlaySoundAtLocation` "/Game/GameAspects/Sounds/EndRoom/Gun_Cue.Gun_Cue" (`SceneComponent.K2_GetComponentLocation` (`self.SkeletalMesh`)))
  (`GameplayStatics.SpawnEmitterAttached` "/Game/StarterContent/Particles/P_Explosion.P_Explosion" (`self.FlashPoint`))
  (for _array_element (`PrimitiveComponent.GetOverlappingComponents` (`self.HitBox`))
    (bind _returnvalue (`KismetSystemLibrary.GetDisplayName` _array_element))
    (`KismetSystemLibrary.PrintString` _returnvalue)
    (if (`KismetStringLibrary.EqualEqual_StrStr` _returnvalue "VRPawn_507.HeadSet GenericHMD")
      (`self.K2_AddActorWorldOffset` (`ActorComponent.GetOwner` _array_element) (-500.0 0.0 0.0) false false))))

(event `/Game/GameAspects/Blueprints/PickupActorInterface.Pickup`
  (params (AttachTo :type "SceneComponent Object Reference"))
  (bind _skeletalmesh (`self.SkeletalMesh`))
  (`PrimitiveComponent.SetSimulatePhysics` (`self.SkeletalMesh`) false)
  (`SceneComponent.K2_AttachToComponent` (`self.SkeletalMesh`) AttachTo "None" "SnapToTarget" "SnapToTarget" "KeepWorld" false)
  (`SceneComponent.K2_SetWorldRotation` _skeletalmesh (`KismetMathLibrary.MakeRotator` (.roll (`SceneComponent.K2_GetComponentRotation` AttachTo)) (- (.pitch (`SceneComponent.K2_GetComponentRotation` AttachTo)) 90.0) (.yaw (`SceneComponent.K2_GetComponentRotation` AttachTo))) false false)
  (`SceneComponent.K2_SetWorldLocation` _skeletalmesh (`KismetMathLibrary.MakeVector` (.x (`SceneComponent.K2_GetComponentLocation` AttachTo)) (+ (.y (`SceneComponent.K2_GetComponentLocation` AttachTo)) 2.5) (- (.z (`SceneComponent.K2_GetComponentLocation` AttachTo)) 1.5)) false false))

(event `/Game/GameAspects/Blueprints/PickupActorInterface.Drop`
  (`PrimitiveComponent.SetSimulatePhysics` (`self.SkeletalMesh`) true)
  (`self.K2_DetachFromActor` "KeepWorld" "KeepWorld" "KeepWorld"))

(fn `UserConstructionScript`)