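; BP_Books_Child is an interactable book prop, a child Blueprint that randomizes its appearance when play begins.
; BeginPlay sets each axis of the static mesh's relative scale to an independent random float between 0 and 1, so books can be non-uniform or nearly flat.
; It then randomly picks one of four colored book meshes: blue, brown, green or red.
; The construction script only calls the parent's.
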(event `self.ReceiveBeginPlay`
  (bind _returnvalue (+ (`KismetMathLibrary.RandomFloat`) 0.0))
  (`SceneComponent.SetRelativeScale3D` (`self.StaticMeshComponent`) (`KismetMathLibrary.MakeVector` _returnvalue _returnvalue _returnvalue))
  (switch `int` (`KismetMathLibrary.RandomInteger` 4)
    (:`0`
      (`StaticMeshComponent.SetStaticMesh` (`self.StaticMeshComponent`) "/Game/Geometry/Meshes/Room03/IO_Books_01_Book_Blue.IO_Books_01_Book_Blue"))
    (:`1`
      (`StaticMeshComponent.SetStaticMesh` (`self.StaticMeshComponent`) "/Game/Geometry/Meshes/Room03/IO_Books_01_Book_Brown.IO_Books_01_Book_Brown"))
    (:`2`
      (`StaticMeshComponent.SetStaticMesh` (`self.StaticMeshComponent`) "/Game/Geometry/Meshes/Room03/IO_Books_01_Book_Green.IO_Books_01_Book_Green"))
    (:`3`
      (`StaticMeshComponent.SetStaticMesh` (`self.StaticMeshComponent`) "/Game/Geometry/Meshes/Room03/IO_Books_01_Book_Red.IO_Books_01_Book_Red"))))

(fn `UserConstructionScript`
  (`parent.UserConstructionScript`))