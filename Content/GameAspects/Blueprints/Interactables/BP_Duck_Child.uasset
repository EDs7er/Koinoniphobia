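; BP_Duck_Child is a grabbable duck interactable that squeaks when a motion controller picks it up.
; On Pickup it plays the squeak at the mesh location, disables physics simulation and attaches its root to the supplied component, keeping world transform.
; On Drop it re-enables physics and detaches.
; Its construction script only runs the parent's.
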(event `/Game/GameAspects/Blueprints/PickupActorInterface.Pickup`
  (params (AttachTo :type "SceneComponent Object Reference"))
  (`GameplayStatics.PlaySoundAtLocation` "/Game/GameAspects/Sounds/Bathroom/Squeaky_Cue.Squeaky_Cue" (`SceneComponent.K2_GetComponentLocation` (`self.StaticMeshComponent`)))
  (`PrimitiveComponent.SetSimulatePhysics` (`self.StaticMeshComponent`) false)
  (`SceneComponent.K2_AttachToComponent` (`self.K2_GetRootComponent`) AttachTo "None" "KeepWorld" "KeepWorld" "KeepWorld" false))

(event `/Game/GameAspects/Blueprints/PickupActorInterface.Drop`
  (`PrimitiveComponent.SetSimulatePhysics` (`self.StaticMeshComponent`) true)
  (`self.K2_DetachFromActor` "KeepWorld" "KeepWorld" "KeepWorld"))

(fn `UserConstructionScript`
  (`parent.UserConstructionScript`))