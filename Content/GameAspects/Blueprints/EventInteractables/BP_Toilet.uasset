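; BP_Toilet is an interactable toilet whose water rises when flushed and which yields a key when plunged.
; Interact checks for a Hand-tagged actor on the handle, plays a sound and, unless already raising, spawns particles and starts the water Level Sequence.
; A Plunger-tagged overlap spawns BP_Key_Child and plays that same sequence in reverse.
; Raising and Falling flags gate both actions; key pickup logic is left disconnected.
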(event `/Game/GameAspects/Blueprints/PhysicInteractables/PhysicObjectInterface.Interact`
  (params (HandLocation :type "Vector Structure") (Component :type "SceneComponent Object Reference"))
  (for _array_element (`PrimitiveComponent.GetOverlappingActors` (`self.HandleCollision`) null)
    (if (`self.ActorHasTag` _array_element "Hand")
      (`GameplayStatics.PlaySoundAtLocation` null (`SceneComponent.K2_GetComponentLocation` (`self.Toilet`)))
      (if (not (`self.Raising?`))
        (`GameplayStatics.SpawnEmitterAtLocation` "/Game/StarterContent/Particles/P_Sparks.P_Sparks" (`SceneComponent.K2_GetComponentLocation` (`self.SpawnPoint`)) (struct) false)
        (bind _returnvalue (`LevelSequencePlayer.CreateLevelSequencePlayer` (`self.WaterRaising`) "/Game/GameAspects/Blueprints/EventInteractables/WaterLevelSequence.WaterLevelSequence"))
        (set `self.Water` _returnvalue)
        (`MovieSceneSequencePlayer.Play` _returnvalue)
        (set `self.Raising?` true)
        (set `self.Falling?` false)))))

(event `self.ReceiveTick`
  (params (DeltaSeconds :type "Float (single-precision)")))

(event `self.ReceiveActorBeginOverlap`
  (params (OtherActor :type "Actor Object Reference"))
  (bind _water (`self.Water`))
  (if (`self.Falling?`)
    _
    (elif (`self.ActorHasTag` OtherActor "Plunger")
      (bind _returnvalue (`|SpawnActorFromClass` "/Game/GameAspects/Blueprints/Interactables/BP_Key_Child.BP_Key_Child_C" (`KismetMathLibrary.MakeTransform` (`SceneComponent.K2_GetComponentLocation` (`self.SpawnPoint`))) "Undefined" "OverrideRootScale"))
      (`MovieSceneSequencePlayer.SetPlayRate` _water 1.0)
      (`MovieSceneSequencePlayer.PlayReverse` _water)
      (`KismetSystemLibrary.PrintString` "Hello")
      (set `self.Falling?` true)
      (set `self.Raising?` false))))

(fn `UserConstructionScript`)