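; BP_MainMenu is a physical main menu with Play, Help, About and Exit buttons, pressed by touching them with a component named IndexSphere.
; Every tick it polls each button's overlapping components and matches that sphere by object name, so actions repeat while contact lasts.
; Play unlocks the BP_Hatch actors tagged Hatch, Help and About call PressHelp and PressAbout, and Exit quits the game.
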(event `self.ReceiveTick`
  (params (DeltaSeconds :type "Float (single-precision)"))
  (`|ExecutionSequence`
    (:`then_0`
      (for _array_element (`PrimitiveComponent.GetOverlappingComponents` (`self.PlayButton`))
        (if (`KismetStringLibrary.EqualEqual_StrStr` (`KismetSystemLibrary.GetObjectName` _array_element) "IndexSphere")
          (bind _outactors (`GameplayStatics.GetAllActorsWithTag` "Hatch"))
          (for _array_element_2 _outactors
            (bind _asbp_hatch (cast `/Game/GameAspects/Blueprints/PhysicInteractables/BP_Hatch` _array_element_2))
            (`/Game/GameAspects/Blueprints/PhysicInteractables/BP_Hatch.Unlock_Hatch` _asbp_hatch)))))
    (:`then_1`
      (for _array_element_3 (`PrimitiveComponent.GetOverlappingComponents` (`self.HelpButton`))
        (if (`KismetStringLibrary.EqualEqual_StrStr` (`KismetSystemLibrary.GetObjectName` _array_element_3) "IndexSphere")
          (`self.PressHelp`))))
    (:`then_2`
      (for _array_element_4 (`PrimitiveComponent.GetOverlappingComponents` (`self.AboutButton`))
        (if (`KismetStringLibrary.EqualEqual_StrStr` (`KismetSystemLibrary.GetObjectName` _array_element_4) "IndexSphere")
          (`self.PressAbout`))))
    (:`then_3`
      (for _array_element_5 (`PrimitiveComponent.GetOverlappingComponents` (`self.ExitButton`))
        (if (`KismetStringLibrary.EqualEqual_StrStr` (`KismetSystemLibrary.GetObjectName` _array_element_5) "IndexSphere")
          (`KismetSystemLibrary.QuitGame` null "Quit"))))))

(fn `UserConstructionScript`)