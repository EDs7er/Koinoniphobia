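; Portrait jigsaw puzzle that drops the portrait and spawns a key once all nine pieces are placed.
; Each Tick scans the Box overlaps for pieces by display name, then releases the motion controller's held item, plays a click and reveals the matching built-in piece.
; Per-piece macros destroy the carried piece by tag after a short delay.
; When all flags are set, physics is enabled on the portrait and a one-time key spawns.
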(event `self.ReceiveTick`
  (params (DeltaSeconds :type "Float (single-precision)"))
  (if (and (and (and (and (`self.Piece1`) (`self.Piece2`)) (and (`self.Piece3`) (`self.Piece4`))) (and (and (`self.Piece5`) (`self.Piece6`)) (and (`self.Piece7`) (`self.Piece8`)))) (`self.Piece9`))
    (if (not (`self.Unlocked`))
      (`PrimitiveComponent.SetSimulatePhysics` (`self.Portrait`) true)
      (`|SpawnActorFromClass` "/Game/GameAspects/Blueprints/Interactables/BP_Key_Child.BP_Key_Child_C" (`KismetMathLibrary.MakeTransform` (`SceneComponent.K2_GetComponentLocation` (`self.SpawnKey`))) "Undefined" "OverrideRootScale")
      (set `self.Unlocked` true))
    (else
      (for _array_element (`PrimitiveComponent.GetOverlappingActors` (`self.Box`) null)
        (`|ExecutionSequence`
          (:`then_0`
            (bind _returnvalue (`KismetSystemLibrary.GetDisplayName` _array_element))
            (if (`KismetStringLibrary.EqualEqual_StrStr` _returnvalue "BP_PuzzlePiece01_Child")
              (`self.DropItem`)
              (`GameplayStatics.SpawnSoundAttached` "/Game/GameAspects/Sounds/Clicker_sounds_Cue.Clicker_sounds_Cue" (`self.Portrait`))
              (set `self.Piece1` true)
              (`SceneComponent.SetVisibility` (`self.Piece01`) true false)
              (`self.DeletePiece01`)))
          (:`then_1`
            (if (`KismetStringLibrary.EqualEqual_StrStr` _returnvalue "BP_PuzzlePiece02_Child")
              (`self.DropItem`)
              (`GameplayStatics.SpawnSoundAttached` "/Game/GameAspects/Sounds/Clicker_sounds_Cue.Clicker_sounds_Cue" (`self.Portrait`))
              (set `self.Piece2` true)
              (`SceneComponent.SetVisibility` (`self.Piece02`) true false)
              (`self.DeletePiece02`)))
          (:`then_2`
            (if (`KismetStringLibrary.EqualEqual_StrStr` _returnvalue "BP_PuzzlePiece03_Child")
              (`self.DropItem`)
              (`GameplayStatics.SpawnSoundAttached` "/Game/GameAspects/Sounds/Clicker_sounds_Cue.Clicker_sounds_Cue" (`self.Portrait`))
              (set `self.Piece3` true)
              (`SceneComponent.SetVisibility` (`self.Piece03`) true false)
              (`self.DeletePiece03`)))
          (:`then_3`
            (if (`KismetStringLibrary.EqualEqual_StrStr` _returnvalue "BP_PuzzlePiece04_Child")
              (`self.DropItem`)
              (`GameplayStatics.SpawnSoundAttached` "/Game/GameAspects/Sounds/Clicker_sounds_Cue.Clicker_sounds_Cue" (`self.Portrait`))
              (set `self.Piece4` true)
              (`SceneComponent.SetVisibility` (`self.Piece04`) true false)
              (`self.DeletePiece04`)))
          (:`then_4`
            (if (`KismetStringLibrary.EqualEqual_StrStr` _returnvalue "BP_PuzzlePiece05_Child")
              (`self.DropItem`)
              (`GameplayStatics.SpawnSoundAttached` "/Game/GameAspects/Sounds/Clicker_sounds_Cue.Clicker_sounds_Cue" (`self.Portrait`))
              (set `self.Piece5` true)
              (`SceneComponent.SetVisibility` (`self.Piece05`) true false)
              (`self.DeletePiece05`)))
          (:`then_5`
            (if (`KismetStringLibrary.EqualEqual_StrStr` _returnvalue "BP_PuzzlePiece06_Child")
              (`self.DropItem`)
              (`GameplayStatics.SpawnSoundAttached` "/Game/GameAspects/Sounds/Clicker_sounds_Cue.Clicker_sounds_Cue" (`self.Portrait`))
              (set `self.Piece6` true)
              (`SceneComponent.SetVisibility` (`self.Piece06`) true false)
              (`self.DeletePiece06`)))
          (:`then_6`
            (if (`KismetStringLibrary.EqualEqual_StrStr` _returnvalue "BP_PuzzlePiece07_Child")
              (`self.DropItem`)
              (`GameplayStatics.SpawnSoundAttached` "/Game/GameAspects/Sounds/Clicker_sounds_Cue.Clicker_sounds_Cue" (`self.Portrait`))
              (set `self.Piece7` true)
              (`SceneComponent.SetVisibility` (`self.Piece07`) true false)
              (`self.DeletePiece07`)))
          (:`then_7`
            (if (`KismetStringLibrary.EqualEqual_StrStr` _returnvalue "BP_PuzzlePiece08_Child")
              (`self.DropItem`)
              (`GameplayStatics.SpawnSoundAttached` "/Game/GameAspects/Sounds/Clicker_sounds_Cue.Clicker_sounds_Cue" (`self.Portrait`))
              (set `self.Piece8` true)
              (`SceneComponent.SetVisibility` (`self.Piece08`) true false)
              (`self.DeletePiece08`)))
          (:`then_8`
            (if (`KismetStringLibrary.EqualEqual_StrStr` _returnvalue "BP_PuzzlePiece09_Child")
              (`self.DropItem`)
              (`GameplayStatics.SpawnSoundAttached` "/Game/GameAspects/Sounds/Clicker_sounds_Cue.Clicker_sounds_Cue" (`self.Portrait`))
              (set `self.Piece9` true)
              (`SceneComponent.SetVisibility` (`self.Piece09`) true false)
              (`self.DeletePiece09`))))))))

(fn `UserConstructionScript`)